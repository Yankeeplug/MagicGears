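; BP_Enemy_base is the base AI enemy character, reused through an object pool and assigned to the Blue or Red team.
; Active resets health, fetches pool and spawner from BP_GameMaster, and caches its team's point of interest.
; Attack plays a swing animation, then after a delay damages the blackboard's PlayerToAttack; its line trace result is unused.
; Lethal damage despawns it to the pool and decrements the spawner's count, ending the wave or game.
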(event Custom|Attack
  (bind _arrow1 (Variables|Default|GetArrow1))
  (bind _returnvalue (Transformation|GetWorldLocation _arrow1))
  ;[1 1 1] animation try to do a notify on the animatiom
  (Collision|LineTraceByChannel _returnvalue (+ (* (Math|Vector|GetForwardVector _arrow1) 1.5e+03) _returnvalue) "TraceTypeQuery2" false 0 "ForDuration")
  (Components|Animation|OverrideAnimationData (Variables|Character|GetMesh) "/Game/animation/goblin/attacking/Heavy_Weapon_Swing__1_.Heavy_Weapon_Swing__1_" true true 0.0 1.0)
  (Utilities|FlowControl|Delay 0.2)
  (Class|BPIBaseStates|DamageTakenEvent(Message) (AI|Components|Blackboard|GetValueasObject (Variables|/Script/AIModule.AIController|GetBlackboard (AI|GetAIController self)) (Variables|Default|GetPlayerToAttack)) (Variables|Default|Getdamage)))

(event EventActive
  (params (ObjectPoolIn :type AC%20Object%20Pool%20Object%20Reference) (CameraVector :type Vector :default "0, 0, 0"))
  (Variables|Default|SetDespawned false)
  (bind _returnvalue (Actor|GetActorOfClass "/Game/GameMaster/BP_GameMaster.BP_GameMaster_C"))
  (Variables|Default|SetObject%20Pool (Variables|/Game/GameMaster/BP_GameMaster.BP_GameMaster_C|GetAC_ObjectPool _returnvalue))
  (Variables|Default|SetSpawner (Variables|/Game/GameMaster/BP_GameMaster.BP_GameMaster_C|GetAC_Spawner _returnvalue))
  (Variables|Default|Sethealth_0 (Variables|Default|GetmaxHealth))
  (Utilities|FlowControl|Delay 0.2)
  (CallFunction|UpdateHealthBar)
  (switch Utilities|FlowControl|Switch|SwitchonE_Team (Variables|Default|GetTEAMOnEnemyBase)
    (:NewEnumerator1
      (bind _returnvalue_2 (Actor|GetActorOfClass "/Game/AI/pointOfIntrestFolder/BP_AIPointOfIntrest_blue.BP_AIPointOfIntrest_blue_C"))
      (Variables|AI|SetAIPointOfIntrest%20blue _returnvalue_2))
    (:NewEnumerator2
      (bind _returnvalue_3 (Actor|GetActorOfClass "/Game/AI/pointOfIntrestFolder/BP_AIPointOfIntrest_red.BP_AIPointOfIntrest_red_C"))
      (Variables|AI|SetAIPointOfIntrestRed _returnvalue_3))))

(fn ConstructionScript)

(fn UpdateHealthBar
  (if (> (Variables|Default|Gethealth_0) 0)
    (bind _asw_aihealth_bar (Utilities|Casting|CastToW_AIHealthBar (UserInterface|GetUserWidgetObject (Variables|Default|GethealthBar)))
      (:then
        (Variables|/Game/UI/Widgets/AI_widgets/W_AIHealthBar.W_AIHealthBar_C|Sethealth _asw_aihealth_bar (/ (Variables|Default|Gethealth_0) (Variables|Default|GetmaxHealth)))
        (return))
      (:CastFailed
        (Development|PrintString "cast failed")))))

(fn Attackable
  (return (Variables|Default|Getattackable?)))

(fn CharaterGroundFriction
  (params (groundFriction :type Float%20%28double-precision%29) (brakingFriction :type Float%20%28double-precision%29))
  (bind _charactermovement (Variables|Character|GetCharacterMovement))
  (Variables|/Script/Engine.CharacterMovementComponent|SetGroundFriction _charactermovement groundFriction)
  (Variables|/Script/Engine.CharacterMovementComponent|SetBrakingFriction _charactermovement brakingFriction)
  (return))

(fn DamageTakenEvent
  (params (damage%20given :type Integer))
  (bind _spawner (Variables|Default|GetSpawner))
  ;[1 0.004751 0] damage
  (Variables|Default|Sethealth_0 (- (Variables|Default|Gethealth_0) damage%20given))
  (if (<= (Variables|Default|Gethealth_0) 0)
    (if (not (Variables|Default|GetDespawned))
      (Variables|Default|SetDespawned true)
      (Default|Despawn (Variables|Default|GetObject%20Pool) self)
      (Variables|/Game/GameMaster/Spawner/AC_Spawner.AC_Spawner_C|SetEnemies _spawner (- (Variables|/Game/GameMaster/Spawner/AC_Spawner.AC_Spawner_C|GetEnemies _spawner) 1))
      (if (<= (Variables|/Game/GameMaster/Spawner/AC_Spawner.AC_Spawner_C|GetEnemies _spawner) 0)
        (Default|EndWave _spawner)
        (if (>= (Variables|/Game/GameMaster/Spawner/AC_Spawner.AC_Spawner_C|GetWaveIndex _spawner) (Variables|/Game/GameMaster/Spawner/AC_Spawner.AC_Spawner_C|GetMaxWaves _spawner))
          (Default|EndGame _spawner))
        (else
          (return (Variables|Default|Gethealth_0)))))
    (else
      (Development|PrintString (Utilities|String|ToString(Integer) (Variables|Default|Gethealth_0)))
      (CallFunction|UpdateHealthBar)
      (return (Variables|Default|Gethealth_0)))))

(fn GettingonMap
  (return false))

(fn Hero
  (return (Variables|Default|GetHero?)))

(fn Minion
  (return (Variables|Default|GetMinion?)))

(fn PointOfIntrest
  (return (Variables|AI|GetAIPointOfIntrest%20blue) (Variables|AI|GetAIPointOfIntrestRed)))

(fn SettingTeam
  (params (team :type E_Team%20Enum :default "NewEnumerator0"))
  (Variables|Default|SetTEAMOnEnemyBase team)
  (return))

(fn SpawnedinAllie
  (return false))

(fn TEAM
  (return (Variables|Default|GetTEAMOnEnemyBase)))