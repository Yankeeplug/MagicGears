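; BP_AIPointOfIntrest_red is a patrol route for AI, defined by the points of a spline component named Route.
; The incrementingPatrol event steps PatrolIndex by Direction and flips Direction at either end of the spline, giving a back-and-forth ping-pong path.
; GetSplineWorldLocation returns the world-space location of the spline point at the current PatrolIndex.
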(event Custom|incrementing%20Patrol
  (bind _output_get (Variables|Default|SetPatrolIndex (+ (Variables|Default|Getdirection) (Variables|Default|GetPatrolIndex))))
  (if (== _output_get (- (Spline|GetNumberOfSplinePoints (Variables|Default|Getroute)) 1))
    (Variables|Default|Setdirection -1)
    (elif (== (Variables|Default|GetPatrolIndex) 0)
      (Variables|Default|Setdirection 1))))

(event EventBeginPlay)

(fn ConstructionScript)

(fn GetSplineWorldLocation
  (return (Spline|GetLocationatSplinePoint (Variables|Default|Getroute) (Variables|Default|GetPatrolIndex) "World")))