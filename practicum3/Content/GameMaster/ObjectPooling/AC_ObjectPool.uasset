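; Object pooling component that serves as the entry point for spawning and despawning pooled actors.
; Spawn lazily creates one BP_Pool per requested actor type, caches it in the Pools map and delegates the spawn to it.
; Despawn returns an actor to the pool referenced by its AC_PoolMember component, or destroys it when that pool reference is unset.
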(fn Spawn
  (params (Actor :type Actor%20Class%20Reference) (Transform :type Transform))
  (bind _pools (Variables|Default|GetPools))
  (if (Utilities|Map|Contains _pools Actor)
    _
    (else
      (bind _returnvalue (Game|SpawnActorfromClass "/Game/GameMaster/ObjectPooling/BP_Pool.BP_Pool_C" (Variables|Default|GetSpawnTransform) "Undefined" "MultiplyWithRoot" 0 0))
      (Utilities|Map|Add _pools Actor _returnvalue)
      (Variables|/Game/GameMaster/ObjectPooling/BP_Pool.BP_Pool_C|SetObjectBlueprint _returnvalue Actor)))
  (bind _spawnedactor (Default|Spawn (.Value (Utilities|Map|Find _pools Actor)) Transform))
  (return _spawnedactor))

(fn Despawn
  (params (Actor :type Actor%20Object%20Reference))
  (bind _returnvalue (Actor|GetComponentbyClass Actor "/Game/GameMaster/ObjectPooling/AC_PoolMember.AC_PoolMember_C"))
  (bind _mypool (Variables|/Game/GameMaster/ObjectPooling/AC_PoolMember.AC_PoolMember_C|GetMyPool _returnvalue))
  (if (== _mypool 0)
    (Actor|DestroyActor Actor)
    (else
      (Default|Despawn _mypool Actor))))