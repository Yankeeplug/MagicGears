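; BP_Pool is an object pool that spawns and recycles actors of a configurable class (ObjectBlueprint).
; Spawn reuses the last entry in InactiveObjects, or creates a counted actor with a pool-member component linked back to the pool.
; It activates and repositions the actor, calling itself again if invalid, without returning that retry's result.
; Despawn only deactivates the root component and stores the actor for reuse.
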(fn ConstructionScript)

(fn Spawn
  (params (Transform :type Transform))
  (bind _inactiveobjects (Variables|Default|GetInactiveObjects))
  (bind _returnvalue (Utilities|Array|LastIndex _inactiveobjects))
  (bind _output (Utilities|Array|Get(acopy) _inactiveobjects _returnvalue))
  (Variables|Default|SetSpawnedActor 0)
  (if (Utilities|Array|IsEmpty _inactiveobjects)
    (bind _returnvalue_2 (Game|SpawnActorfromClass (Variables|Default|GetObjectBlueprint) Transform "Undefined" "MultiplyWithRoot" 0 0))
    (bind _output_get (Variables|Default|SetSpawnedActor _returnvalue_2))
    (AddComponent|AddACPoolMember _output_get self)
    (Math|Integer|IncrementInt (Variables|Default|GetObjectCount)
      (:%20%20
        _))
    (else
      (Variables|Default|SetSpawnedActor _output)
      (Utilities|Array|RemoveItem _inactiveobjects _output)))
  (Utilities|IsValid (Variables|Default|GetSpawnedActor)
    (:Is%20Valid
      (Components|Activation|SetActive (Variables|/Script/Engine.Actor|GetRootComponent (Variables|Default|GetSpawnedActor)) true false)
      (Transformation|SetActorTransform (Variables|Default|GetSpawnedActor) Transform)
      (return (Variables|Default|GetSpawnedActor)))
    (:Is%20Not%20Valid
      (CallFunction|Spawn Transform))))

(fn Despawn
  (params (Actor :type Actor%20Object%20Reference))
  (Components|Activation|SetActive (Variables|/Script/Engine.Actor|GetRootComponent Actor) false false)
  (Utilities|Array|Add (Variables|Default|GetInactiveObjects) Actor))