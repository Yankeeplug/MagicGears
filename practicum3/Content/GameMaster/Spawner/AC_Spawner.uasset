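; AC_Spawner is a wave spawner, apparently an actor component, that is only partly wired up.
; On BeginPlay it caches the object pool from BP_GameMaster and the row names of DT_Waves.
; Unconnected logic checks the wave index, calling an empty Win at the limit or looping over the current wave's EnemyData.
; The pool Spawn call for each enemy type is also disconnected, so nothing spawns.
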(event EventBeginPlay
  (bind _returnvalue (Actor|GetActorOfClass "/Game/GameMaster/BP_GameMaster.BP_GameMaster_C"))
  (Variables|Default|SetObjectPool (Variables|/Game/GameMaster/BP_GameMaster.BP_GameMaster_C|GetAC_ObjectPool _returnvalue))
  (bind _outrownames (DataTable|GetDataTableRowNames "/Game/GameMaster/Spawner/DT_Waves.DT_Waves"))
  (Variables|Default|SetWaves _outrownames))

(fn Win)