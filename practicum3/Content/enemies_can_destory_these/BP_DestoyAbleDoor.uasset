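; BP_DestoyAbleDoor is a door actor with health and a health bar widget, apparently meant for enemies to destroy.
; On BeginPlay it sends the Health/MaxHealth ratio to its W_AIHealthBar, provided Health is above zero.
; Combat query functions return fixed defaults, including false for Hero, Minion and Attackable.
; DamageEvent only returns zero, so the file shows no damage or destruction logic.
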(event EventBeginPlay
  (CallFunction|UpdateHealthBar))

(event Collision|EventActorBeginOverlap
  (params (OtherActor :type Actor%20Object%20Reference)))

(event EventTick
  (params (DeltaSeconds :type Float%20%28single-precision%29)))

(fn ConstructionScript)

(fn DamageEvent
  (params (damage%20taken :type Integer))
  (return 0))

(fn Hero
  (return false))

(fn Minion
  (return false))

(fn Attackable
  (return false))

(fn TEAM
  (return "NewEnumerator0"))

(fn PointOfIntrest
  (return 0 0))

(fn UpdateHealthBar
  (if (> (Variables|Default|Gethealth) 0)
    (bind _asw_aihealth_bar (Utilities|Casting|CastToW_AIHealthBar (UserInterface|GetUserWidgetObject (Variables|Default|GethealthBar)))
      (:then
        (Variables|/Game/Widgets/AI_widgets/W_AIHealthBar.W_AIHealthBar_C|Sethealth _asw_aihealth_bar (/ (Variables|Default|Gethealth) (Variables|Default|Getmax%20health)))
        (return))
      (:CastFailed
        (Development|PrintString "cast failed")))))