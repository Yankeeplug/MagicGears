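; Player character component for building traps: previews, places and removes the traps listed in the character's TrapsForMatch array.
; Mouse wheel cycles the trap index, with an extra slot past the end for attack mode; a delay loop from BeginPlay switches build mode to match.
; In build mode, Tick traces from the follow camera on the trap's channel to position a preview mesh, and input spawns its Blueprint there.
; Another trace destroys actors tagged "buildable".
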(event Custom|preview%20loop
  (bind _follow_camera (Variables|Default|GetFollow%20Camera))
  (bind _returnvalue (Transformation|GetWorldLocation _follow_camera))
  ;[0 0.3828 0.05525] line trace
  (bind (_outhit _returnvalue_2) (Collision|LineTraceByChannel _returnvalue (+ _returnvalue (* (Math|Vector|GetForwardVector _follow_camera) (Variables|Default|Getline%20trace%20distance))) (.layertracechannel (Utilities|Struct|BreakS_Trap (Utilities|Array|Get(acopy) (Variables|Default|GetTraps%20for%20Match%28BPC_buildSystem%29) (Variables|Default|Getbuildable%20index)))) false 0 "ForDuration"))
  (if _returnvalue_2
    (bind _output_get (Variables|Default|SetHit%20Component (.HitComponent (Collision|BreakHitResult _outhit))))
    (Variables|Default|SetHit%20Actor (.HitActor (Collision|BreakHitResult _outhit)))
    (Utilities|FlowControl|Sequence
      (:then_0
        (Utilities|FlowControl|DoOnce false
          (:Completed
            (bind _returnvalue_3 (Game|AddComponentbyClass (Variables|Default|Getplayer%20BP) "/Script/Engine.StaticMeshComponent" false (Variables|Default|Getbuild%20preview%20transform)))
            (bind _output_get_2 (Variables|Default|SetPreview%20mesh _returnvalue_3))
            (Components|StaticMesh|SetStaticMesh _output_get_2 (.mesh (Utilities|Struct|BreakS_Trap (Utilities|Array|Get(acopy) (Variables|Default|GetTraps%20for%20Match%28BPC_buildSystem%29) (Variables|Default|Getbuildable%20index)))))
            (Rendering|Material|SetMaterial (Variables|Default|GetPreview%20mesh) 0 "/Game/materials/M_preview.M_preview")
            (Collision|SetCollisionEnabled (Variables|Default|GetPreview%20mesh) "NoCollision"))))
      (:then_1
        ;;[1 1 1] trap transform
        (bind _output_get_3 (Variables|Default|Setbuild%20preview%20transform (Math|Transform|MakeTransform (.Location (Collision|BreakHitResult _outhit)) (Variables|/Script/Engine.SceneComponent|GetRelativeRotation _output_get) "1.000000,1.000000,1.000000")))
        (Transformation|SetWorldTransform (Variables|Default|GetPreview%20mesh) _output_get_3 false false)))))

(event Custom|reset%20build%20mode
  ;[0 0.3828 0.05525] line trace
  (Utilities|FlowControl|DoOnce false) ; enters at Reset
)

(event Custom|stop%20build%20mode
  ;[1 1 1] to stop build mode
  ;[0.8496 0.244 1] on and off build
  (Variables|Default|SetInBuildMode false)
  (bind _preview_mesh (Variables|Default|GetPreview%20mesh)
    (:then
      (Components|StaticMesh|SetStaticMesh _preview_mesh 0)
      (Variables|Default|SetPreview%20mesh 0)
      (CallFunction|ResetBuildMode))
    (:else)))

(event Custom|start%20build%20mode
  ;[0.8496 0.244 1] on and off build
  (Variables|Default|SetInBuildMode true))

(event Input|EnhancedActionEvents|EnhancedInputActionIA_buildMode
  (params (ActionValue :type Boolean) (ElapsedSeconds :type Float%20%28double-precision%29) (TriggeredSeconds :type Float%20%28double-precision%29) (InputAction :type Input%20Action%20Object%20Reference :default "/Game/ThirdPerson/Input/Actions/IA_buildMode.IA_buildMode"))
  (:Started
    ;[0.8496 0.244 1] on and off build
    ;;[1 1 1] stop build mode
    (if (not (Variables|Default|GetInBuildMode))
      (Variables|Default|SetInBuildMode true)
      (else
        (Variables|Default|SetInBuildMode false)
        (bind _preview_mesh (Variables|Default|GetPreview%20mesh)
          (:then
            (Components|StaticMesh|SetStaticMesh _preview_mesh 0)
            (Variables|Default|SetPreview%20mesh 0)
            (CallFunction|ResetBuildMode))
          (:else))))))

(event Input|EnhancedActionEvents|EnhancedInputActionIA_placeBuild
  (params (ActionValue :type Boolean) (ElapsedSeconds :type Float%20%28double-precision%29) (TriggeredSeconds :type Float%20%28double-precision%29) (InputAction :type Input%20Action%20Object%20Reference :default "/Game/ThirdPerson/Input/Actions/IA_placeBuild.IA_placeBuild"))
  (:Started
    (if (Variables|Default|GetInBuildMode)
      (bind _buildable (Class|BPITrap|Buildable(Message) (Variables|Default|GetHit%20Actor)))
      (if (not _buildable)
        (bind _returnvalue (Game|SpawnActorfromClass (.blueprint (Utilities|Struct|BreakS_Trap (Utilities|Array|Get(acopy) (Variables|Default|GetTraps%20for%20Match%28BPC_buildSystem%29) (Variables|Default|Getbuildable%20index)))) (Variables|Default|Getbuild%20preview%20transform) "AdjustIfPossibleButDontSpawnIfColliding" "MultiplyWithRoot" 0 0))))))

(event Input|EnhancedActionEvents|EnhancedInputActionIA_destoryTrap
  (params (ActionValue :type Boolean) (ElapsedSeconds :type Float%20%28double-precision%29) (TriggeredSeconds :type Float%20%28double-precision%29) (InputAction :type Input%20Action%20Object%20Reference :default "/Game/ThirdPerson/Input/Actions/IA_destoryTrap.IA_destoryTrap"))
  (bind _follow_camera (Variables|Default|GetFollow%20Camera))
  (bind _returnvalue (Transformation|GetWorldLocation _follow_camera))
  (:Started
    (bind (_outhit _returnvalue_2) (Collision|LineTraceByChannel _returnvalue (+ _returnvalue (* (Math|Vector|GetForwardVector _follow_camera) (Variables|Default|Getline%20trace%20distance))) "TraceTypeQuery1" false 0 "ForDuration"))
    (if _returnvalue_2
      (if (Actor|ActorHasTag (.HitActor (Collision|BreakHitResult _outhit)) "buildable")
        (Actor|DestroyActor (.HitActor (Collision|BreakHitResult _outhit)))))))

(event EventBeginPlay
  (Utilities|FlowControl|Delay 1.0)
  (bind _asbp_third_person_character (Utilities|Casting|CastToBP_ThirdPersonCharacter (Components|GetOwner)))
  (bind _output_get (Variables|Default|Setplayer%20BP _asbp_third_person_character))
  (Variables|Default|SetFollow%20Camera (Variables|/Game/ThirdPerson/Blueprints/BP_ThirdPersonCharacter.BP_ThirdPersonCharacter_C|GetFollowCamera _asbp_third_person_character))
  ;[1 1 1] acts as a list of all the traps in Datatables (cant change the data table
  (bind _output_get_2 (Variables|Default|SetTraps%20for%20Match%28BPC_buildSystem%29 (Variables|/Game/ThirdPerson/Blueprints/BP_ThirdPersonCharacter.BP_ThirdPersonCharacter_C|GetTrapsForMatch _output_get)))
  (for _array_element _output_get_2
    (Development|PrintString (.name (Utilities|Struct|BreakS_Trap _array_element)))
    (Variables|Default|Setbuildable%20index (Utilities|Array|Length (Variables|Default|GetTraps%20for%20Match%28BPC_buildSystem%29)))
    (Development|PrintString (Utilities|String|ToString(Integer) (Utilities|Array|Length (Variables|Default|GetTraps%20for%20Match%28BPC_buildSystem%29))))
    (if (< (Variables|Default|Getbuildable%20index) (Utilities|Array|Length (Variables|Default|GetTraps%20for%20Match%28BPC_buildSystem%29))) :!label _label
      (CallFunction|StartBuildMode)
      (else
        (CallFunction|StopBuildMode)))
    (Utilities|FlowControl|Delay 0.01)
    (goto _label)))

(event EventTick
  (params (DeltaSeconds :type Float%20%28single-precision%29))
  (if (Variables|Default|GetInBuildMode)
    (CallFunction|PreviewLoop)))

(event Input|MouseEvents|MouseWheelDown
  (params (Key :type Key%20Structure :default "None"))
  (:Pressed
    (Variables|Default|Setbuildable%20index (- (Variables|Default|Getbuildable%20index) 1))
    (if (< (Variables|Default|Getbuildable%20index) 0)
      (Variables|Default|Setbuildable%20index (Utilities|Array|Length (Variables|Default|GetTraps%20for%20Match%28BPC_buildSystem%29)))
      (else
        (bind _preview_mesh (Variables|Default|GetPreview%20mesh)
          (:then
            (Components|StaticMesh|SetStaticMesh _preview_mesh 0)
            (Variables|Default|SetPreview%20mesh 0)
            (CallFunction|ResetBuildMode))
          (:else))))))

(event Input|MouseEvents|MouseWheelUp
  (params (Key :type Key%20Structure :default "None"))
  (:Pressed
    (if (> (Variables|Default|Getbuildable%20index) (Utilities|Array|Length (Variables|Default|GetTraps%20for%20Match%28BPC_buildSystem%29)))
      (Variables|Default|Setbuildable%20index 0)
      (else
        (Variables|Default|Setbuildable%20index (Math|Integer|Clamp(Integer) (+ (Variables|Default|Getbuildable%20index) 1) 0 (Utilities|Array|Length (Variables|Default|GetTraps%20for%20Match%28BPC_buildSystem%29))))
        (bind _preview_mesh (Variables|Default|GetPreview%20mesh)
          (:then
            (Components|StaticMesh|SetStaticMesh _preview_mesh 0)
            (Variables|Default|SetPreview%20mesh 0)
            (CallFunction|ResetBuildMode))
          (:else))))))