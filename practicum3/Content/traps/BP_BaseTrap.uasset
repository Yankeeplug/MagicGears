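; Base trap Blueprint that supplies a countdown cooldown and default answers to unit-classification queries.
; The cooldown event refills its count from the configured number when depleted, then loops through a one-second Delay, decrementing and printing the count until it runs out.
; Query functions report it as non-attackable and non-hero, ignore damage, and expose buildable, minion and team variables, with team set by the spawner.
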(event Custom|cooldown%20Event
  (if (> (Variables|Default|Getcooldown%20count) 0)
    _
    (else
      (Variables|Default|Setcooldown%20count (Variables|Default|GetcooldownNumber))))
  (bind _output_get (Variables|Default|Setcooldown%20count (- (Variables|Default|Getcooldown%20count) 1) :!label _label))
  (Development|PrintString (Utilities|String|ToString(Integer) _output_get))
  (Utilities|FlowControl|Delay 1.0)
  (if (> (Variables|Default|Getcooldown%20count) 0)
    (goto _label)))

(fn ConstructionScript)

(fn Attackable
  (return false))

(fn Buildable
  (return (Variables|Default|Getbuildable?)))

(fn DamageTakenEvent
  (params (damage%20given :type Integer))
  (return 0))

(fn GettingonMap
  (return false))

(fn Hero
  (return false))

(fn Minion
  (return (Variables|Default|Getnot%20a%20minoin)))

(fn PointOfIntrest
  (return 0 0))

(fn SpawnedinAllie
  (return false))

(fn TEAM
  (return (Variables|Default|GetTeamOnTrap)))