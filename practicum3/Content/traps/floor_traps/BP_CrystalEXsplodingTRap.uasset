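; Single-use crystal floor trap that damages minions stepping onto it.
; On overlap it runs the parent handler, then identifies minions through a MinionMessage interface call.
; A minion receives BaseDamage via DamageTakenEventMessage, and the trap destroys itself after a short delay.
; The graph itself contains no explosion effect or area damage, only the hit on the overlapping actor.
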(event EventBeginPlay
  (|CallParentFunction) ; This node is disabled and will not be called.\nDrag off pins to build functionality.
)

(event Collision|EventActorBeginOverlap
  (params (OtherActor :type Actor%20Object%20Reference))
  (|CallParentFunction OtherActor)
  (bind _minion (Class|BPIBaseStates|Minion(Message) OtherActor))
  (if _minion
    (Class|BPIBaseStates|DamageTakenEvent(Message) OtherActor (Variables|Default|Getbase_damage))
    (Utilities|FlowControl|Delay 0.5)
    (Actor|DestroyActor)))

(event EventTick
  (params (DeltaSeconds :type Float%20%28single-precision%29))
  (|CallParentFunction DeltaSeconds) ; This node is disabled and will not be called.\nDrag off pins to build functionality.
)

(fn ConstructionScript
  (|CallParentFunction))