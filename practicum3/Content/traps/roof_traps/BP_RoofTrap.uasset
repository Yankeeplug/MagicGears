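; BP_RoofTrap is a roof trap Blueprint that detects minions entering its capsule; this graph only tracks targets and contains no attack logic.
; Begin overlap queries the actor's minion and team messages, stores any minion as AttackTarget, but sets HaveTarget only when its team differs from TeamOnTrap.
; End overlap clears both for the current target, with debug prints.
; The trap itself reports a fixed team and non-minion status.
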(event OnComponentBeginOverlap(Capsule)
  (params (OverlappedComponent :type Primitive%20Component%20Object%20Reference) (OtherActor :type Actor%20Object%20Reference) (OtherComp :type Primitive%20Component%20Object%20Reference) (OtherBodyIndex :type Integer) (bFromSweep :type Boolean) (SweepResult :type Hit%20Result%20Structure%20%28by%20ref%29))
  (bind _minion (Class|BPIBaseStates|Minion(Message) OtherActor))
  (if _minion
    (bind _team (Class|BPIBaseStates|TEAM(Message) OtherActor))
    (bind _output_get (Variables|Default|SetattackTarget OtherActor))
    (Development|PrintString (Utilities|GetDisplayName _output_get))
    (if (not (Utilities|Enum|Equal(Enum) _team (Variables|Default|GetTeamOnTrap)))
      (Variables|Default|SethaveTarget true))))

(event OnComponentEndOverlap(Capsule)
  (params (OverlappedComponent :type Primitive%20Component%20Object%20Reference) (OtherActor :type Actor%20Object%20Reference) (OtherComp :type Primitive%20Component%20Object%20Reference) (OtherBodyIndex :type Integer))
  (if (== OtherActor (Variables|Default|GetattackTarget))
    (bind _output_get (Variables|Default|SetattackTarget 0))
    (Development|PrintString (Utilities|GetDisplayName _output_get))
    (Variables|Default|SethaveTarget false)))

(event EventBeginPlay
  (|CallParentFunction) ; This node is disabled and will not be called.\nDrag off pins to build functionality.
)

(event Collision|EventActorBeginOverlap
  (params (OtherActor :type Actor%20Object%20Reference))
  (|CallParentFunction OtherActor) ; This node is disabled and will not be called.\nDrag off pins to build functionality.
)

(event EventTick
  (params (DeltaSeconds :type Float%20%28single-precision%29))
  (|CallParentFunction DeltaSeconds) ; This node is disabled and will not be called.\nDrag off pins to build functionality.
)

(fn ConstructionScript
  (|CallParentFunction))

(fn TEAM
  (return "NewEnumerator0"))

(fn Minion
  (return false))