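; BP_ArrowWall is a wall trap that fires a projectile when a minion overlaps it.
; Actor overlap calls MinionMessage on the other actor and, on a true result, spawns a base projectile at the Arrow component through a DoOnce.
; Any end overlap on Box_0 destroys the stored projectile and resets the DoOnce to rearm the trap.
; Its own Minion function returns NotAMinoin.
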(event OnComponentEndOverlap(Box_0)
  (params (OverlappedComponent :type Primitive%20Component%20Object%20Reference) (OtherActor :type Actor%20Object%20Reference) (OtherComp :type Primitive%20Component%20Object%20Reference) (OtherBodyIndex :type Integer))
  (Actor|DestroyActor (Variables|Default|Getprojectile))
  (Utilities|FlowControl|DoOnce false) ; enters at Reset
)

(event EventBeginPlay
  (|CallParentFunction) ; This node is disabled and will not be called.\nDrag off pins to build functionality.
)

(event Collision|EventActorBeginOverlap
  (params (OtherActor :type Actor%20Object%20Reference))
  (|CallParentFunction OtherActor)
  (bind _minion (Class|BPIBaseStates|Minion(Message) OtherActor))
  (if _minion
    (Utilities|FlowControl|DoOnce false
      (:Completed
        (bind _returnvalue (Game|SpawnActorfromClass "/Game/traps/TrapProjectiles/BP_baseProjectile.BP_baseProjectile_C" (Math|Conversions|ToTransform(Vector) (Transformation|GetWorldLocation (Variables|Default|GetArrow))) "Undefined" "MultiplyWithRoot" 0 0))
        (Variables|Default|Setprojectile _returnvalue)))))

(event EventTick
  (params (DeltaSeconds :type Float%20%28single-precision%29))
  (|CallParentFunction DeltaSeconds) ; This node is disabled and will not be called.\nDrag off pins to build functionality.
)

(fn ConstructionScript
  (|CallParentFunction))

(fn Minion
  (return (Variables|Default|Getnot%20a%20minoin)))